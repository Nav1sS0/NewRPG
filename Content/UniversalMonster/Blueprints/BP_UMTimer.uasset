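; Short-lived Universal Monster helper actor that runs an attack's timed effect: damage over time or a special trace attack.
; On the server, a timer either hits the Instigator for Timer attacks or starts a trace for other attack types.
; Traces interpolate location and radius, instantly or over time, becoming expanding AOEs when start and end locations match.
; Hits pass optional line-of-sight and once-per-actor filters before reaching UniversalMonster's HitEvent.
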(event `self.ReceiveDestroyed`
  (`KismetSystemLibrary.K2_ClearAndInvalidateTimerHandle` (`self.Timer`))
  (`KismetSystemLibrary.K2_ClearAndInvalidateTimerHandle` (`self.SpecialTimer`)))

(event `DamageOverTime`
  (bind _instigator (`self.Instigator`))
  (bind _returnvalue (`self.K2_GetActorLocation` _instigator))
  ;[1 1 1] DoT
  (`/Game/UniversalMonster/Blueprints/BP_UniversalMonster.HitEvent` :`self` (`self.UniversalMonster`) :`Attack` (`self.Attack`) :`Timer` self :`Hit Result` (`GameplayStatics.MakeHitResult` true false 0.0 0.0 _returnvalue _returnvalue (0.0 0.0 1.0) (0.0 0.0 1.0) null _instigator)))

(event `SpecialTrace`
  (bind _returnvalue (`self.K2_GetActorLocation`))
  (bind _universalmonster (`self.UniversalMonster`))
  (bind _nextalpha (`self.NextAlpha`))
  (bind _currentalpha (`self.CurrentAlpha`))
  (bind _aoetrace (`self.AOETrace`))
  (bind ((`Special_59_1C0D91494ADBA7743FBA7D8EA42AE8DD` _special) (`Trace_131_8FC178054F11AD0076B3078EA6F165C7` _trace)) (break `/Game/UniversalMonster/Blueprints/Structs/S_Attack` (`self.Attack`)))
  (bind ((`StartLocation_42_F13652B2414F09E9D2A12EB055FD27E3` _startlocation) (`EndLocation_39_2A4962864A94209CA44840B14015AA9F` _endlocation) (`StartRadius_40_8F2D30B84A6157AA5D967FA9FFD0AD12` _startradius) (`EndRadius_41_FAEDD29A4D260CD08AD9DB9A436038A5` _endradius)) (break `/Game/UniversalMonster/Blueprints/Structs/S_Special` _special))
  (bind _returnvalue_2 (select `bool` (`/Game/UniversalMonster/Blueprints/BP_UniversalMonster.bEnableDebugging` (`self.UniversalMonster`)) :`true` "ForDuration" :!type "EDrawDebugTrace Enum"))
  (bind _returnvalue_3 (+ _returnvalue _endlocation))
  (bind _returnvalue_4 (+ _returnvalue _startlocation))
  (bind _returnvalue_5 (select `bool` true :`false` (`|MakeArray` null :!type "Actor Object Reference") :`true` (`|MakeArray` _universalmonster (`/Game/UniversalMonster/Blueprints/BP_UniversalMonster.Actor` _universalmonster) self :!type "Actor Object Reference")))
  (bind _returnvalue_6 (`KismetMathLibrary.VLerp` _returnvalue_4 _returnvalue_3 _currentalpha))
  ;[1 1 1] Special Attack Trace
  (bind _hitresults (`/Game/UniversalMonster/Blueprints/BP_UniversalMonster.CustomTrace` :`self` (`self.UniversalMonster`) :`TraceType` "NewEnumerator3" :`Trace` _trace :`Start` _returnvalue_6 :`End` (select `bool` _aoetrace :`false` (`KismetMathLibrary.VLerp` _returnvalue_4 _returnvalue_3 _nextalpha) :`true` (+ _returnvalue_6 0.01)) :`Radius` (`KismetMathLibrary.Lerp` _startradius _endradius (select `bool` _aoetrace :`false` _currentalpha :`true` _nextalpha)) :`ActorsToIgnore` _returnvalue_5 :`DrawDebugType` _returnvalue_2))
  (for _array_element _hitresults
    (bind _output_get (set `self.CurrentHit` _array_element))
    (bind (_bblockinghit _binitialoverlap _time _distance _location _impactpoint _normal _impactnormal _physmat _hitactor) (`GameplayStatics.BreakHitResult` _output_get))
    (if _bblockinghit
      (if (`.PassThroughEnvironment?_57_4C6AB1614244EEF06847E594530030D2` (break `/Game/UniversalMonster/Blueprints/Structs/S_TraceInfo` (`.Trace_131_8FC178054F11AD0076B3078EA6F165C7` (break `/Game/UniversalMonster/Blueprints/Structs/S_Attack` (`self.Attack`)))))
        (if (not (and (`.OneHitPerActor?_40_0120D9244E9E912FC3F525B9AFF42611` (break `/Game/UniversalMonster/Blueprints/Structs/S_TraceInfo` (`.Trace_131_8FC178054F11AD0076B3078EA6F165C7` (break `/Game/UniversalMonster/Blueprints/Structs/S_Attack` (`self.Attack`))))) (`KismetArrayLibrary.Array_Contains` (`self.HitTargets`) _hitactor))) :!label _label
          (`KismetArrayLibrary.Array_AddUnique` (`self.HitTargets`) _hitactor)
          (`/Game/UniversalMonster/Blueprints/BP_UniversalMonster.HitEvent` :`self` (`self.UniversalMonster`) :`Attack` (`self.Attack`) :`Timer` self :`Hit Result` (`self.CurrentHit`)))
        (else
          (bind _outhit (`KismetSystemLibrary.LineTraceSingle` (`self.K2_GetActorLocation`) _impactpoint "TraceTypeQuery1" false _returnvalue_5 _returnvalue_2 true (struct :`R` 1.0 :`A` 1.0) (struct :`G` 1.0 :`A` 1.0) 0.5))
          (if (== _hitactor (`.HitActor` (`GameplayStatics.BreakHitResult` _outhit)))
            (goto _label)))))))

(event `self.ReceiveBeginPlay`
  (bind ((`Duration_58_233A2ED2431E48B4EAFA7FA66C12CBAD` _duration) (`Time_57_174F12DE41446B9B91124490D6D997D8` _time) (`Looping?_55_25ED9B294D1423FBC99038901666B1C3` _looping_) (`InitialStartDelay_54_3D8564FE41FCF0A1B1FEBAA37418AC16` _initialstartdelay) (`InitialStartDelayVariance_53_00EDE9414B1C06E39F7E4898C746E114` _initialstartdelayvariance)) (break `/Game/UniversalMonster/Blueprints/Structs/S_Special` (`.Special_59_1C0D91494ADBA7743FBA7D8EA42AE8DD` (break `/Game/UniversalMonster/Blueprints/Structs/S_Attack` (`self.Attack`)))))
  (`self.SetLifeSpan` (`KismetMathLibrary.FMax` _duration 0.01))
  (`/Engine/EditorBlueprintResources/ActorMacros.Switch Has Authority`
    (:`Authority`
      (bind _returnvalue (`KismetSystemLibrary.K2_SetTimerDelegate` (delegate `TimerEvent`) (`KismetMathLibrary.FMax` _time) _looping_ (`KismetMathLibrary.FMax` _initialstartdelay) (`KismetMathLibrary.FMax` _initialstartdelayvariance)))
      (set `self.Timer` _returnvalue)
      (if (or (<= _time 0.0) (< _initialstartdelay 0.0))
        (`self.TimerEvent`)))))

(event `TimerEvent`
  (switch `/Game/UniversalMonster/Blueprints/Enums/E_AttackType` (`.Type_25_2F2358B84E0FCF1CD97742BC251D25B9` (break `/Game/UniversalMonster/Blueprints/Structs/S_Attack` (`self.Attack`)))
    (:`NewEnumerator0`
      (`self.SpecialAttack` :!label _label_2))
    (:`NewEnumerator1`
      (goto _label_2))
    (:`NewEnumerator2`
      (goto _label_2))
    (:`NewEnumerator3`
      (`self.DamageOverTime`))))

(event `SpecialAttack`
  (bind ((`Special_59_1C0D91494ADBA7743FBA7D8EA42AE8DD` _special) (`Trace_131_8FC178054F11AD0076B3078EA6F165C7` _trace)) (break `/Game/UniversalMonster/Blueprints/Structs/S_Attack` (`self.Attack`)))
  (bind ((`InstantTrace?_49_188B1EC947C62DA5D3BE86834F854B99` _instanttrace_) (`TraceDuration_46_510FD8774B44C745B5A1E89502CDA4A8` _traceduration) (`StartLocation_42_F13652B2414F09E9D2A12EB055FD27E3` _startlocation) (`EndLocation_39_2A4962864A94209CA44840B14015AA9F` _endlocation) (`StartRadius_40_8F2D30B84A6157AA5D967FA9FFD0AD12` _startradius) (`EndRadius_41_FAEDD29A4D260CD08AD9DB9A436038A5` _endradius)) (break `/Game/UniversalMonster/Blueprints/Structs/S_Special` _special))
  (bind _output_get (set `self.AOETrace` (== _startlocation _endlocation :`ErrorTolerance` 0.01)))
  (if _instanttrace_
    (if (or _output_get (`KismetMathLibrary.NearlyEqual_FloatFloat` _startradius _endradius 0.01))
      (set `self.CurrentAlpha` 0.0)
      (set `self.NextAlpha` 1.0)
      (`self.SpecialTrace`)
      (`KismetArrayLibrary.Array_Clear` (`self.HitTargets`))
      (else
        (bind _output_get_2 (set `self.NumTraces` (`KismetMathLibrary.FTrunc` (* (`.TracesPerSecond_21_6007138B443CDF35746244BC53FD451D` (break `/Game/UniversalMonster/Blueprints/Structs/S_TraceInfo` _trace)) _traceduration))))
        (for _index (range (+ _output_get_2 1))
          (bind _returnvalue (`KismetMathLibrary.Conv_IntToDouble` _output_get_2))
          (set `self.CurrentAlpha` (/ (`KismetMathLibrary.Conv_IntToDouble` _index) _returnvalue))
          (set `self.NextAlpha` (/ (`KismetMathLibrary.FMin` (`KismetMathLibrary.Conv_IntToDouble` (+ _index 1)) (+ _returnvalue 0.01)) _returnvalue))
          (`self.SpecialTrace`))
        (`KismetArrayLibrary.Array_Clear` (`self.HitTargets`))))
    (else
      (set `self.StartTime` (`KismetSystemLibrary.GetGameTimeInSeconds`))
      (bind _returnvalue_2 (`KismetSystemLibrary.K2_SetTimerDelegate` (delegate `TraceTimer`) (`KismetMathLibrary.FMax` (/ 1.0 (`.TracesPerSecond_21_6007138B443CDF35746244BC53FD451D` (break `/Game/UniversalMonster/Blueprints/Structs/S_TraceInfo` (`.Trace_131_8FC178054F11AD0076B3078EA6F165C7` (break `/Game/UniversalMonster/Blueprints/Structs/S_Attack` (`self.Attack`))))))) true))
      (set `self.SpecialTimer` _returnvalue_2))))

(event `TraceTimer`
  (bind ((`Special_59_1C0D91494ADBA7743FBA7D8EA42AE8DD` _special) (`Trace_131_8FC178054F11AD0076B3078EA6F165C7` _trace)) (break `/Game/UniversalMonster/Blueprints/Structs/S_Attack` (`self.Attack`)))
  (bind _returnvalue (- (`KismetSystemLibrary.GetGameTimeInSeconds`) (`self.StartTime`)))
  (bind ((`TraceDuration_46_510FD8774B44C745B5A1E89502CDA4A8` _traceduration)) (break `/Game/UniversalMonster/Blueprints/Structs/S_Special` _special))
  (if (>= _returnvalue _traceduration)
    (`KismetSystemLibrary.K2_ClearAndInvalidateTimerHandle` (`self.SpecialTimer`))
    (`KismetArrayLibrary.Array_Clear` (`self.HitTargets`))
    (else
      (set `self.CurrentAlpha` (/ _returnvalue _traceduration))
      (set `self.NextAlpha` (/ (+ _returnvalue (`KismetMathLibrary.FMax` (/ 1.0 (`.TracesPerSecond_21_6007138B443CDF35746244BC53FD451D` (break `/Game/UniversalMonster/Blueprints/Structs/S_TraceInfo` _trace))))) _traceduration))
      (`self.SpecialTrace`))))

(fn `UserConstructionScript`)