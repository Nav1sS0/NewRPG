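; Projectile for UniversalMonster attacks, with movement, bounce and optional timed homing on the monster's current target configured from Attack data.
; On authority, it converts sphere, capsule and box components under Arrow into BP_UMTrace components.
; A looping timer sweeps each trace from its previous to current position, reporting once per target per trace to the monster's HitEvent.
; It expires on lifespan, despawn range or non-pass-through hits.
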(event `self.ReceiveDestroyed`
  (`KismetSystemLibrary.K2_ClearAndInvalidateTimerHandle` (`self.TraceTimer`)))

(event `self.ReceiveBeginPlay`
  (bind _projectilemovement (`self.ProjectileMovement`))
  (bind ((`Projectile_24_61D994CE43075C87919BBC930340A5BD` _projectile) (`Trace_131_8FC178054F11AD0076B3078EA6F165C7` _trace)) (break `/Game/UniversalMonster/Blueprints/Structs/S_Attack` (`self.Attack`)))
  (bind _currenttarget (`/Game/UniversalMonster/Blueprints/BP_UniversalMonster.CurrentTarget` (`self.UniversalMonster`)))
  (bind ((`HomingDuration_120_EC2176B4436ADF0E5F5C3DB9D3A4759B` _homingduration)) (break `/Game/UniversalMonster/Blueprints/Structs/S_Projectile` (`.Projectile_24_61D994CE43075C87919BBC930340A5BD` (break `/Game/UniversalMonster/Blueprints/Structs/S_Attack` (`self.Attack`)))))
  (bind ((`Homing?_67_6E473F754A3F458A25E811974817C302` _homing_) (`LifeSpan_52_75212FF2473557DE410EF19A68D6CC80` _lifespan)) (break `/Game/UniversalMonster/Blueprints/Structs/S_Projectile` _projectile))
  (`/Engine/EditorBlueprintResources/ActorMacros.Switch Has Authority`
    (:`Authority`
      (`self.SetTraces`)
      (for _array_element (`self.K2_GetComponentsByClass` "/Game/UniversalMonster/Blueprints/BP_UMTrace.BP_UMTrace_C")
        (`BlueprintMapLibrary.Map_Add` (`self.Traces`) _array_element (`SceneComponent.K2_GetComponentLocation` _array_element)))
      (if _homing_
        (`/Engine/EditorBlueprintResources/StandardMacros.IsValid` _currenttarget
          (:`Is Valid`
            (set `ProjectileMovementComponent.HomingTargetComponent` (`Actor.RootComponent` _currenttarget) (`self.ProjectileMovement`)))
          (:`Is Not Valid`
            _)))
      (`self.SetLifeSpan` _lifespan)
      (bind _returnvalue (`KismetSystemLibrary.K2_SetTimerDelegate` (delegate `Trace`) (`KismetMathLibrary.FMax` 0.0 (/ 1.0 (`.TracesPerSecond_21_6007138B443CDF35746244BC53FD451D` (break `/Game/UniversalMonster/Blueprints/Structs/S_TraceInfo` _trace)))) true))
      (set `self.TraceTimer` _returnvalue)
      (if (> _homingduration 0.0)
        (`KismetSystemLibrary.Delay` _homingduration)
        (set `ProjectileMovementComponent.bIsHomingProjectile` false _projectilemovement)
        (set `ProjectileMovementComponent.HomingTargetComponent` null _projectilemovement)))))

(event `Trace`
  (`/Engine/EditorBlueprintResources/StandardMacros.IsValid` (`self.UniversalMonster`)
    (:`Is Valid`
      (`self.ProjectileTrace`)
      (if (>= (`KismetMathLibrary.Vector_Distance` (`self.Origin`) (`self.K2_GetActorLocation`)) (`.DespawnRange_88_8F5392E24E14964FF78BC596CC84410C` (break `/Game/UniversalMonster/Blueprints/Structs/S_Projectile` (`.Projectile_24_61D994CE43075C87919BBC930340A5BD` (break `/Game/UniversalMonster/Blueprints/Structs/S_Attack` (`self.Attack`))))))
        (`self.SetLifeSpan` 0.01)))
    (:`Is Not Valid`
      (`KismetSystemLibrary.K2_ClearAndInvalidateTimerHandle` (`self.TraceTimer`)))))

(event `ProjectileTrace`
  (bind _currenttrace (`self.CurrentTrace`))
  (bind _currenttrace_2 (`self.CurrentTrace`))
  (bind _currenttrace_3 (`self.CurrentTrace`))
  (bind _hittargets (`self.HitTargets`))
  (bind _universalmonster (`self.UniversalMonster`))
  (bind _returnvalue (`SceneComponent.K2_GetComponentScale` _currenttrace_2))
  (bind _returnvalue_2 (`SceneComponent.K2_GetComponentLocation` _currenttrace_2))
  (bind _z (.z _returnvalue))
  ;[1 1 1] Projectile Trace
  (bind _keys (`BlueprintMapLibrary.Map_Keys` (`self.Traces`)))
  (for _array_element _keys
    (bind _output_get (set `self.CurrentTrace` _array_element))
    (`/Engine/EditorBlueprintResources/StandardMacros.IsValid` _output_get
      (:`Is Valid`
        (bind _hitresults (`/Game/UniversalMonster/Blueprints/BP_UniversalMonster.CustomTrace` (`self.UniversalMonster`) (`/Game/UniversalMonster/Blueprints/BP_UMTrace.TraceType` _currenttrace_2) (`.Trace_131_8FC178054F11AD0076B3078EA6F165C7` (break `/Game/UniversalMonster/Blueprints/Structs/S_Attack` (`self.Attack`))) (`BlueprintMapLibrary.Map_Find` (`self.Traces`) _currenttrace_2) _returnvalue_2 (* (`/Game/UniversalMonster/Blueprints/BP_UMTrace.BoxExtent` _currenttrace_2) _returnvalue) (`SceneComponent.K2_GetComponentRotation` _currenttrace_2) (* (`/Game/UniversalMonster/Blueprints/BP_UMTrace.Radius` _currenttrace_2) _z) (* (`/Game/UniversalMonster/Blueprints/BP_UMTrace.HalfHeight` _currenttrace_2) _z) (`|MakeArray` (`/Game/UniversalMonster/Blueprints/BP_UniversalMonster.Actor` _universalmonster) _universalmonster self :!type "Actor Object Reference") (select `bool` (`/Game/UniversalMonster/Blueprints/BP_UniversalMonster.bEnableDebugging` (`self.UniversalMonster`)) :`true` "ForDuration" :!type "EDrawDebugTrace Enum") (struct :`R` 1.0 :`A` 1.0) (struct :`G` 1.0 :`A` 1.0) 0.5))
        (for _array_element_2 _hitresults
          (bind _output_get_2 (set `self.CurrentHit` _array_element_2))
          (bind _output_get_3 (set `self.HitTargets` (`.HitTargets_4_E935E5F7457C35FE1C070486A8AEAA1D` (break `/Game/UniversalMonster/Blueprints/Structs/S_HitTargets` (`BlueprintMapLibrary.Map_Find` (`self.TraceTargets`) (`self.CurrentTrace`))))))
          (bind (_shouldhit_ _shouldpassthrough_ _hitactor) (`/Game/UniversalMonster/Blueprints/BPFL_UMFunctions.ShouldHit` _output_get_2 (`self.Attack`) (`self.UniversalMonster`) _output_get_3))
          (if (not _shouldpassthrough_)
            (`self.SetLifeSpan` 0.01))
          (if _shouldhit_
            (`KismetArrayLibrary.Array_AddUnique` _hittargets _hitactor)
            (`BlueprintMapLibrary.Map_Add` (`self.TraceTargets`) _currenttrace (make `/Game/UniversalMonster/Blueprints/Structs/S_HitTargets` _hittargets))
            (`/Game/UniversalMonster/Blueprints/BP_UniversalMonster.HitEvent` :`self` (`self.UniversalMonster`) :`Attack` (`self.Attack`) :`UM Trace` _currenttrace :`Projectile` self :`Hit Result` (`self.CurrentHit`))))
        (`/Engine/EditorBlueprintResources/StandardMacros.IsValid` _currenttrace_3
          (:`Is Valid`
            (`BlueprintMapLibrary.Map_Add` (`self.Traces`) _currenttrace_3 _returnvalue_2)))))))

(fn `SetTraces`
  (locals (LocalComponent :type "SceneComponent Object Reference") (LocalTrace :type "/Game/UniversalMonster/Blueprints/BP_UMTrace Object Reference"))
  (bind _localcomponent (`local.LocalComponent`))
  (for _array_element (`SceneComponent.GetChildrenComponents` (`self.Arrow`) true)
    (bind _output_get (set `local.LocalComponent` _array_element))
    (bind _assphere_collision (cast `SphereComponent` _output_get)
      (:`then`
        (bind _returnvalue (`AddComponent|NODE_AddBP_UMTrace-0` :`bManualAttachment` true :`RelativeTransform` (`SceneComponent.GetRelativeTransform` _assphere_collision) :`NotifyName` (`KismetSystemLibrary.GetObjectName` _assphere_collision) :`TraceType` "NewEnumerator3" :`Radius` (`SphereComponent.SphereRadius` _assphere_collision)))
        (set `local.LocalTrace` _returnvalue))
      (:`CastFailed`
        (bind _ascapsule_collision (cast `CapsuleComponent` (`local.LocalComponent`))
          (:`then`
            (bind _returnvalue_2 (`AddComponent|NODE_AddBP_UMTrace-1` :`bManualAttachment` true :`RelativeTransform` (`SceneComponent.GetRelativeTransform` _ascapsule_collision) :`NotifyName` (`KismetSystemLibrary.GetObjectName` _ascapsule_collision) :`TraceType` "NewEnumerator1" :`Radius` (`CapsuleComponent.CapsuleRadius` _ascapsule_collision) :`HalfHeight` (`CapsuleComponent.CapsuleHalfHeight` _ascapsule_collision)))
            (set `local.LocalTrace` _returnvalue_2))
          (:`CastFailed`
            (bind _asbox_collision (cast `BoxComponent` (`local.LocalComponent`)))
            (bind _returnvalue_3 (`AddComponent|NODE_AddBP_UMTrace-2` :`bManualAttachment` true :`RelativeTransform` (`SceneComponent.GetRelativeTransform` _asbox_collision) :`NotifyName` (`KismetSystemLibrary.GetObjectName` _asbox_collision) :`BoxExtent` (`BoxComponent.BoxExtent` _asbox_collision)))
            (set `local.LocalTrace` _returnvalue_3)))))
    (`SceneComponent.K2_AttachToComponent` (`local.LocalTrace`) (`SceneComponent.GetAttachParent` _localcomponent) (`SceneComponent.GetAttachSocketName` _localcomponent) "KeepRelative" "KeepRelative" "KeepRelative" true)))

(fn `UserConstructionScript`
  (bind _projectilemovement (`self.ProjectileMovement`))
  (bind ((`InitialSpeed_60_725F54E546353FE8E11D4586C3A97E86` _initialspeed) (`MaxSpeed_63_A3AFCF4C437C5285202B558BC45A2B9E` _maxspeed) (`Gravity_25_F0E7C354442137D4D03DEBAD1C6D3CBC` _gravity) (`Bounciness_24_127C6D6A49AD139199C5DAB77E6BF251` _bounciness) (`Friction_23_8A7038764F2FBDCDAE956C83EF182766` _friction) (`Homing?_67_6E473F754A3F458A25E811974817C302` _homing_) (`HomingAcceleration_65_649154CC4D7EE6E9AE2AF6A1C7362449` _homingacceleration)) (break `/Game/UniversalMonster/Blueprints/Structs/S_Projectile` (`.Projectile_24_61D994CE43075C87919BBC930340A5BD` (break `/Game/UniversalMonster/Blueprints/Structs/S_Attack` (`self.Attack`)))))
  (set `self.Origin` (`self.K2_GetActorLocation`))
  (set `MovementComponent.Velocity` (* (`self.Direction`) _initialspeed) _projectilemovement)
  (set `ProjectileMovementComponent.MaxSpeed` _maxspeed _projectilemovement)
  (set `ProjectileMovementComponent.ProjectileGravityScale` _gravity _projectilemovement)
  (bind _output_get (set `ProjectileMovementComponent.Bounciness` _bounciness _projectilemovement))
  (set `ProjectileMovementComponent.bShouldBounce` (> _output_get 0.0) _projectilemovement)
  (set `ProjectileMovementComponent.Friction` _friction _projectilemovement)
  (set `ProjectileMovementComponent.bIsHomingProjectile` _homing_ _projectilemovement)
  (set `ProjectileMovementComponent.HomingAccelerationMagnitude` _homingacceleration _projectilemovement))