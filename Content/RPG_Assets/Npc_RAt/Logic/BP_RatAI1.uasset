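; BP_RatAI1 is a rat enemy character that chases and melee-attacks the third-person player and can be killed.
; Pawn sensing sets a blackboard flag on seeing the player, and damage drains health until a death animation plays and the actor is destroyed.
; AttachPlayer sphere-traces forward, checks the player's block, then plays a random attack or none, slowing movement before ramping speed back up.
; The block check reads the cast result before that cast runs.
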(event `self.Damage`
  (params (Damage :type "Float (double-precision)"))
  ;[1 1 1] Dammage AI
  (if (not (`self.Death`))
    (`GameplayStatics.PlaySound2D` "/Game/RPG_Assets/Sound/Sound_Rat/rat_hit_01.rat_hit_01" 1.0 1.0 0.0 null null)
    (bind _output_get (set `self.Health` (`KismetMathLibrary.FMax` 0.0 (`KismetMathLibrary.FMax` (- (`self.Health`) Damage)))))
    (`KismetSystemLibrary.PrintString` (`KismetStringLibrary.Conv_DoubleToString` _output_get))
    (if (== (`self.Health`) 0.0)
      (if (not (`self.Death`))
        (`/Engine/EditorBlueprintResources/StandardMacros.DoOnce` false
          (:`Completed`
            (set `self.Death` true)
            (`SkeletalMeshComponent.PlayAnimation` (`self.Mesh`) "/Game/RPG_Assets/Npc_RAt/Animation/SM_Rat_Anim_death.SM_Rat_Anim_death" false)
            (`NavMovementComponent.StopActiveMovement` (`self.CharacterMovement`))
            (`ActorComponent.SetActive` (`self.CharacterMovement`) false false)
            (`KismetSystemLibrary.Delay` 3.0)
            (`self.K2_DestroyActor`)))))))

(event `AttachPlayer`
  (bind _returnvalue (`self.K2_GetActorLocation`))
  ;[1 1 1] Dammage Player
  (if (not (`self.Death`))
    (set `CharacterMovementComponent.MaxWalkSpeed` 150.0 (`self.CharacterMovement`))
    (bind (_outhit _returnvalue_2) (`KismetSystemLibrary.SphereTraceSingleForObjects` :`Start` _returnvalue :`End` (+ _returnvalue (* (`KismetMathLibrary.GetForwardVector` (`self.K2_GetActorRotation`)) 300.0)) :`Radius` 50.0 :`ObjectTypes` (`|MakeArray` "ObjectTypeQuery3" :!type "EObjectTypeQuery Enum") :`DrawDebugType` "ForDuration"))
    (if _returnvalue_2
      (if (`/Game/RPG_Assets/CharacterMainGui/Mesh_MainGui/BP_ThirdPersonCharacter.b_IsBlock` (stale _asbp_third_person_character))
        (`KismetSystemLibrary.PrintString` "Block Sucses")
        (else
          (bind (_bblockinghit _binitialoverlap _time _distance _location _impactpoint _normal _impactnormal _physmat _hitactor) (`GameplayStatics.BreakHitResult` _outhit))
          (bind _asbp_third_person_character (cast `/Game/RPG_Assets/CharacterMainGui/Mesh_MainGui/BP_ThirdPersonCharacter` _hitactor))
          (bind _output_get (set `self.BlockAnimRandom` (`KismetMathLibrary.RandomInteger` 4)))
          (switch `int` _output_get
            (:`0`
              (`GameplayStatics.PlaySound2D` "/Game/RPG_Assets/Sound/Sound_Rat/rat_attack_01.rat_attack_01" 1.0 1.0 0.0 null null)
              (`self.PlayAnimMontage` "/Game/RPG_Assets/Npc_RAt/Animation/Anim_attach/SM_Rat_Anim_attack_1_Montage.SM_Rat_Anim_attack_1_Montage")
              (message `/Game/RPG_Assets/Game_info/BPI_Damage.Damage` _hitactor 6.0))
            (:`1`
              (`GameplayStatics.PlaySound2D` "/Game/RPG_Assets/Sound/Sound_Rat/rat_attack_02.rat_attack_02" 1.0 1.0 0.0 null null)
              (`self.PlayAnimMontage` "/Game/RPG_Assets/Npc_RAt/Animation/Anim_attach/SM_Rat_Anim_attack_2_Montage.SM_Rat_Anim_attack_2_Montage")
              (message `/Game/RPG_Assets/Game_info/BPI_Damage.Damage` _hitactor 12.0))
            (:`2`
              (`GameplayStatics.PlaySound2D` "/Game/RPG_Assets/Sound/Sound_Rat/rat_attack_03.rat_attack_03" 1.0 1.0 0.0 null null)
              (`self.PlayAnimMontage` "/Game/RPG_Assets/Npc_RAt/Animation/Anim_attach/SM_Rat_Anim_attack_3_Montage.SM_Rat_Anim_attack_3_Montage")
              (message `/Game/RPG_Assets/Game_info/BPI_Damage.Damage` _hitactor 16.0)))
          (`KismetSystemLibrary.Delay` 1.5)
          (set `CharacterMovementComponent.MaxWalkSpeed` 270.0 (`self.CharacterMovement`))
          (`KismetSystemLibrary.Delay` 1.5)
          (set `CharacterMovementComponent.MaxWalkSpeed` 350.0 (`self.CharacterMovement`))
          (`KismetSystemLibrary.Delay` 1.5)
          (set `CharacterMovementComponent.MaxWalkSpeed` 600.0 (`self.CharacterMovement`)))))))

(event `self.PawnSensing.OnSeePawn`
  (params (Pawn :type "Pawn Object Reference"))
  ;[1 1 1] Run Player
  (if (`self.Death`)
    (`BlackboardComponent.SetValueAsBool` (`AIBlueprintHelperLibrary.GetBlackboard` (`AIBlueprintHelperLibrary.GetAIController` self)) "HasSenPlayer?" false)
    (else
      (cast `/Game/RPG_Assets/CharacterMainGui/Mesh_MainGui/BP_ThirdPersonCharacter` Pawn)
      (`BlackboardComponent.SetValueAsBool` (`AIBlueprintHelperLibrary.GetBlackboard` (`AIBlueprintHelperLibrary.GetAIController` self)) "HasSenPlayer?" true))))

(fn `UserConstructionScript`)